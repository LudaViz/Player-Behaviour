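; BP_Holdable is a held item, apparently a base class, that attaches to the instigator character's right hand.
; On BeginPlay it sends its stance through the player animation interface and triggers EquipItem on ABP_Manny; destruction sends a fixed stance.
; Holdable interface functions return its stance and placeholder defaults for actions, ammo, crosshair and left-hand IK, while hit and shoot events are empty.
; An IsLocal helper checks for a locally controlled owning PlayerController.
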(event EventBeginPlay
  (bind _returnvalue (Game|GetInstigator))
  (Class|BPIPlayerAnimation|BPIPlayerAnimationSetStance(Message) _returnvalue (Variables|Default|GetStance))
  (bind _ascharacter (Utilities|Casting|CastToCharacter _returnvalue))
  (Transformation|AttachComponentToComponent (Variables|/Script/Engine.Character|GetMesh _ascharacter) "hand_r" "KeepRelative" "KeepRelative" "KeepRelative" true)
  (bind _asabp_manny (Utilities|Casting|CastToABP_Manny (Components|SkeletalMesh|GetAnimInstance (Variables|/Script/Engine.Character|GetMesh _ascharacter))))
  (Default|EquipItem _asabp_manny))

(event EventDestroyed
  (Class|BPIPlayerAnimation|BPIPlayerAnimationSetStance(Message) (Game|GetInstigator) "NewEnumerator2"))

(event EventBPIHoldableonHit)

(event EventBPIHoldableonShoot
  (params (Intensity :type Float%20%28double-precision%29)))

(fn ConstructionScript)

(fn IsLocal
  (Utilities|FlowControl|Sequence
    (:then_0
      (bind _asplayer_controller (Utilities|Casting|CastToPlayerController (Components|GetOwner)))
      (if (Pawn|IsLocalController _asplayer_controller)
        (return true)))
    (:then_1
      (return false))))

(fn BPIHoldableCallHoldableAction
  (params (Action :type Name :default "None"))
  (return false))

(fn BPIHoldableGetAmmoData
  (return false 0))

(fn BPIHoldableGetCrosshairData
  (return (Utilities|Struct|MakeS_Holdable_Crosshair false 16.0 3e+01)))

(fn BPIHoldableGetLeftHandIKWorldTransform
  (return "0, 0, 0"))

(fn BPIHoldableGetStance
  (return (Variables|Default|GetStance)))