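; BP_LootItem is a world pickup that adds its item to the interacting player's inventory.
; BeginPlay looks up ItemID, async-loads the mesh, enables physics on the collision cube and colors a light by rarity, destroying itself on invalid data.
; Interaction interface functions supply a count-and-name prompt and pass ItemID and ItemData to the player's inventory component, destroying the actor if added.
; Tick spins the mesh by a fixed, frame-rate-dependent step.
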(event EventBeginPlay
  (bind _item_id (Variables|Default|GetItem%20ID))
  ;[1 1 1] Check item existence, if does not exist destroy
  (bind (_item_exists _item_full_data) (CallFunction|GetItemDatafromItemID _item_id))
  (if _item_exists
    ;[1 1 1] Async Load Static mesh and set it
    (bind _output_get (Variables|Default|SetItem%20Full%20Data _item_full_data))
    (bind _object (Utilities|AsyncLoadAsset (.ItemMesh (Utilities|Struct|BreakS_InventorySystem_FullItemData _output_get)))
      (:Completed
        (bind _asstatic_mesh (Utilities|Casting|CastToStaticMesh _object))
        (Components|StaticMesh|SetStaticMesh (Variables|Default|GetItem%20Static%20Mesh) _asstatic_mesh)
        (Utilities|IsValid _asstatic_mesh
          (:Is%20Valid
            (Physics|SetSimulatePhysics (Variables|Default|GetCollisionCube) true)
            (Rendering|Components|Light|SetLightColor (Variables|Default|GetRarity%20LIght) (CallFunction|GetColorfromItemRarity (Utilities|Struct|BreakS_InventorySystem_FullItemData (Variables|Default|GetItem%20Full%20Data))) true))
          (:Is%20Not%20Valid
            (Development|PrintString (Utilities|String|Append "Non-existent static mesh on Item ID " (Utilities|String|ToString(Name) (Variables|Default|GetItem%20ID))) true true "(R=1.000000,G=0.000000,B=0.026519,A=1.000000)" 1e+01)
            (Actor|DestroyActor)))))
    (else
      (Actor|DestroyActor)
      (Development|PrintString (Utilities|String|Append "Item with ID does not exist: " (Utilities|String|ToString(Name) _item_id) ", called from: " (Utilities|GetDisplayName self)) true true "(R=1.000000,G=0.000000,B=0.026519,A=1.000000)" 1e+01))))

(event EventBPIInteractionSystemInteract
  (params (Executed%20by%20Player%20Controller :type Player%20Controller%20Object%20Reference))
  ;[1 1 1] Get Inventory Component from Executing interaction controller and try to add item
  (bind _inventory_comp_reference (Class|BPISimpleInventorySystem|BPISimpleInventorySystemGetInventoryComponent(Message) Executed%20by%20Player%20Controller))
  (Utilities|IsValid _inventory_comp_reference
    (:Is%20Valid
      (bind _success (Default|AddItem _inventory_comp_reference (Variables|Default|GetItem%20ID) (Variables|Default|GetItem%20Data)))
      ;[1 1 1] If added, remove item
      (if _success
        (Actor|DestroyActor)))))

(event EventTick
  (params (DeltaSeconds :type Float%20%28single-precision%29))
  ;[1 1 1] Rotate Item Effect
  (Transformation|AddLocalRotation (Variables|Default|GetItem%20Static%20Mesh) "0.000000,1.000000,0.000000" false false))

(fn ConstructionScript)

(fn BPIInteractionSystemCanInteract
  (return true))

(fn BPIInteractionSystemGetCurrentLocalInteractionActor
  (return 0))

(fn BPIInteractionSystemGetPrompt
  (return (Utilities|String|Append "Pickup " (Utilities|String|ToString(Integer) (.ItemCount (Utilities|Struct|BreakS_InventorySystem_ItemData (Variables|Default|GetItem%20Data)))) "x " (Utilities|String|ToString(Name) (.ItemName (Utilities|Struct|BreakS_InventorySystem_FullItemData (Variables|Default|GetItem%20Full%20Data)))))))