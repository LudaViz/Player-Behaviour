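; Zombie enemy character running BT_Zombie with random health, targeting living players through AI perception.
; Server pushes target and distance to the Blackboard, dropping dead or distant targets.
; Damage turns it toward the attacker; at zero health, IsAlive's RepNotify ragdolls it, stops AI logic and sets a lifespan.
; Multicast attack, hit-flash reaction and corpse-loot events are empty, with their sphere-trace damage, montage and loot logic left disconnected.
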(event OnTargetPerceptionUpdated(AIPerception)
  (params (Actor :type Actor%20Object%20Reference) (Stimulus :type AI%20Stimulus%20Structure))
  ;[1 0.2338 0.3517] On Perception Updated
  (CallFunction|SetCurrentTarget Actor))

(event Custom|MULTICAST%20On%20Damage
  ;[1 1 1] Networked on Damage
)

(event Custom|MULTICAST%20Aattack
  ;[1 1 1] Networked on attack, play montage and apply damage after some time
)

(event EventBPIInteractionSystemInteract
  (params (Executed%20by%20Player%20Controller :type Player%20Controller%20Object%20Reference))
  ;[1 0.3454 0.6771] On Interacted, get if dead, and open stash if possible
)

(event EventTick
  (params (DeltaSeconds :type Float%20%28single-precision%29))
  ;[1 1 1] Update Current target, when exceeds 1800 distance, abandin target
  (|CallParentFunction DeltaSeconds)
  (Networking|SwitchHasAuthority
    (:Authority
      (bind _current_target (Variables|Default|GetCurrent%20Target)
        (:then
          (bind _isalive (Class|BPIPlayerStats|BPIPlayerStatsIsAlive(Message) _current_target))
          (AI|Components|Blackboard|SetValueasFloat (AI|GetBlackboard (AI|GetAIController self)) (Utilities|Name|MakeLiteralName "TargetDistance") (Transformation|GetDistanceTo _current_target))
          (if (or (> (Transformation|GetDistanceTo _current_target) 1.8e+03) (not _isalive))
            (CallFunction|SetCurrentTarget)))
        (:else)))))

(event EventPossessed
  (params (NewController :type Controller%20Object%20Reference))
  ;[1 1 1] Start Behavior
  (|CallParentFunction NewController)
  (bind _asaicontroller (Utilities|Casting|CastToAIController NewController))
  (AI|RunBehaviorTree _asaicontroller "/Game/Dreamrise_SMSK/Blueprints/AI/BT_Zombie.BT_Zombie")
  (Utilities|FlowControl|Sequence
    (:then_0
      ;[1 1 1] Set Random Health
      (Variables|Default|SetHealth (Math|Random|RandomFloatinRange 1e+02 2e+02)))
    (:then_1
      ;[1 1 1] Update reference of self in Blackboard
      (AI|Components|Blackboard|SetValueasObject (AI|GetBlackboard (AI|GetAIController self)) (Utilities|Name|MakeLiteralName "SelfActor") self))))

(event Game|Damage|EventAnyDamage
  (params (Damage :type Float%20%28single-precision%29) (DamageType :type Damage%20Type%20Object%20Reference) (InstigatedBy :type Controller%20Object%20Reference) (DamageCauser :type Actor%20Object%20Reference))
  ;[1 1 1] On Damage Taken
  (bind _output_get (Variables|Default|SetHealth (Math|Float|Clamp(Float) (- (Variables|Default|GetHealth) Damage) 0.0 1e+03)))
  (if (<= _output_get 0.0)
    (Variables|Default|SetbIsAlive false)
    (else
      (CallFunction|MULTICASTonDamage)
      (Transformation|SetActorRotation (Math|Rotator|MakeRotator 0.0 0.0 (.Yaw (Math|Rotator|BreakRotator (Math|Rotator|FindLookatRotation (Transformation|GetActorLocation) (Transformation|GetActorLocation DamageCauser)))))))))

(fn ConstructionScript
  ;[1 0.04352 0.06342] Create dynamic material for zombie for hit effect
  (bind _returnvalue (Rendering|Material|CreateDynamicMaterialInstance "/Game/Dreamrise_SMSK/Characters/UE4_Manny/Materials/MI_Zombie.MI_Zombie" "None" "None" :!class /Script/Engine.KismetMaterialLibrary))
  (bind _output_get (Variables|Default|SetDynamic%20Zombie%20Material _returnvalue))
  (Rendering|Material|SetMaterial (Variables|Character|GetMesh) 0 _output_get))

(fn OnRepBIsAlive
  (bind _mesh (Variables|Character|GetMesh))
  (if (not (Variables|Default|GetbIsAlive))
    (Utilities|FlowControl|Sequence
      (:then_0
        (Collision|SetCollisionResponsetoChannel (Variables|Collision|GetCapsuleComponent) "ECC_Pawn" "ECR_Ignore")
        (Collision|SetCollisionEnabled _mesh "QueryAndPhysics")
        (Collision|SetCollisionObjectType _mesh "ECC_PhysicsBody")
        (Collision|SetCollisionResponsetoChannel _mesh "ECC_WorldStatic" "ECR_Block")
        (Physics|SetSimulatePhysics _mesh true)
        (Actor|SetLifeSpan 1.2e+02))
      (:then_1
        (Networking|SwitchHasAuthority
          (:Authority
            (AI|Logic|StopLogic (Variables|/Script/AIModule.AIController|GetBrainComponent (AI|GetAIController self)) "")))))))

(fn ApplyDamageAroundZombie
  (bind _returnvalue (Transformation|GetActorLocation))
  (bind _outhits (Collision|MultiSphereTraceByChannel _returnvalue (+ (* (Transformation|GetActorForwardVector) (Math|Float|MakeLiteralFloat 1.2e+02)) _returnvalue) 9e+01 "TraceTypeQuery1" false 0 "None"))
  (for _array_element _outhits
    (if (and (not (Utilities|Set|Contains (LocalVariables|GetL%20Actors) (.HitActor (Collision|BreakHitResult _array_element)))) (!= (Utilities|GetClass self) (Utilities|GetClass (.HitActor (Collision|BreakHitResult _array_element)))))
      (Effects|SpawnEmitteratLocation "/Game/Dreamrise_SMSK/Assets/FX/P_ImpactStuff.P_ImpactStuff" (.ImpactPoint (Collision|BreakHitResult _array_element)) "0, 0, 0" "1.000000,1.000000,1.000000" true "AutoRelease")
      (Utilities|Set|Add (LocalVariables|GetL%20Actors) (.HitActor (Collision|BreakHitResult _array_element)))
      (Networking|SwitchHasAuthority
        (:Authority
          (Game|Damage|ApplyPointDamage (.HitActor (Collision|BreakHitResult _array_element)) 2e+01 (Transformation|GetActorLocation) (Collision|MakeHitResult false false 0.0 0.0 "0, 0, 0" "0, 0, 0" "0,0,1" "0,0,1" 0 0) (AI|GetAIController self) self)))))
  (return))

(fn SetCurrentTarget
  (params (Current%20Target :type Actor%20Object%20Reference))
  (Utilities|FlowControl|Sequence
    (:then_0
      (Networking|SwitchHasAuthority
        (:Authority
          (Utilities|IsValid Current%20Target
            (:Is%20Valid
              (bind _asbp_smsk_player_character (Utilities|Casting|CastToBP_SMSK_PlayerCharacter Current%20Target))
              (bind _isalive (Default|BPIPlayerStatsIsAlive _asbp_smsk_player_character))
              (if _isalive
                (bind _output_get (Variables|Default|SetCurrent%20Target Current%20Target :!label _label))
                (AI|Components|Blackboard|SetValueasObject (AI|GetBlackboard (AI|GetAIController self)) (Utilities|Name|MakeLiteralName "TargetActor") _output_get)))
            (:Is%20Not%20Valid
              (goto _label))))))
    (:then_1
      (return))))

(fn SetIsHit
  (params (bIsHit :type Boolean))
  (Utilities|FlowControl|Sequence
    (:then_0
      (Variables|Default|SetbIsHit bIsHit)
      (Networking|SwitchHasAuthority
        (:Authority
          (AI|Components|Blackboard|SetValueasBool (AI|GetBlackboard (AI|GetAIController self)) (Utilities|Name|MakeLiteralName "bIsHit") false))))
    (:then_1
      (return))))

(fn BPIAIInterfaceCallAIAction
  (params (Action :type Name :default "None"))
  (switch name Action
    (:Default
      (return false))
    (:Attack
      (CallFunction|MULTICASTAattack)
      (return true))))

(fn BPIInteractionSystemCanInteract
  (return (<= (Variables|Default|GetHealth) 0.0)))

(fn BPIInteractionSystemGetCurrentLocalInteractionActor
  (return 0))

(fn BPIInteractionSystemGetPrompt
  (return "Loot Dead Zombie"))