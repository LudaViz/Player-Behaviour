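; BP_Holdable_Food is a held food item that the player eats through the holdable primary action.
; Each Start Primary flip-flops between starting and cancelling a timed eat, with a loading widget and eating sound.
; SERVEREat runs the timer, whose completion removes one item from the owner's inventory, adds health to the instigator on success, and destroys the actor.
; Destruction also clears the widget and sound.
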(event Custom|Exec%20Eat
  (Utilities|FlowControl|FlipFlop
    (:A
      (bind _returnvalue (UserInterface|CreateWidget "/Game/Dreamrise_SMSK/Blueprints/Widgets/W_Loading.W_Loading_C" 0 2.0))
      (bind _output_get (Variables|Default|SetWidget _returnvalue))
      (UserInterface|Viewport|AddtoViewport _output_get 0)
      (CallFunction|SERVEREat true)
      (bind _returnvalue_2 (Audio|SpawnSound2D "/Game/Dreamrise_SMSK/Audio/WAV_Eating.WAV_Eating" 1.0 1.0 0.0 0))
      (Variables|Default|SetEat%20Sound _returnvalue_2))
    (:B
      (CallFunction|SERVEREat false)
      (Utilities|FlowControl|Sequence
        (:then_0
          (bind _widget (Variables|Default|GetWidget)
            (:then
              (Widget|RemovefromParent _widget))
            (:else)))
        (:then_1
          (bind _eat_sound (Variables|Default|GetEat%20Sound)
            (:then
              (Audio|Components|Audio|Stop _eat_sound))
            (:else)))))))

(event Custom|SERVER%20Eat
  (params (Toggle :type Boolean))
  (if Toggle
    (bind _returnvalue (Utilities|Time|SetTimerbyEvent (delegate Custom|Eat) 2.0))
    (else
      (Utilities|Time|ClearandInvalidateTimerbyHandle _returnvalue))))

(event Custom|Eat
  (Utilities|FlowControl|Sequence
    (:then_0
      (bind _inventory_comp_reference (Class|BPISimpleInventorySystem|BPISimpleInventorySystemGetInventoryComponent(Message) (Components|GetOwner)))
      (bind _success (Default|RemoveItem _inventory_comp_reference (Variables|Default|GetItem%20ID) 1))
      (if _success
        (Class|BPIPlayerStats|BPIPlayerStatsAddHealth(Message) (Game|GetInstigator) 12.0)))
    (:then_1
      (Actor|DestroyActor))))

(event EventBeginPlay
  (|CallParentFunction) ; This node is disabled and will not be called.\nDrag off pins to build functionality.
)

(event Collision|EventActorBeginOverlap
  (params (OtherActor :type Actor%20Object%20Reference)))

(event EventTick
  (params (DeltaSeconds :type Float%20%28single-precision%29)))

(event EventDestroyed
  (|CallParentFunction)
  (Utilities|FlowControl|Sequence
    (:then_0
      (bind _widget (Variables|Default|GetWidget)
        (:then
          (Widget|RemovefromParent _widget))
        (:else)))
    (:then_1
      (bind _eat_sound (Variables|Default|GetEat%20Sound)
        (:then
          (Audio|Components|Audio|Stop _eat_sound))
        (:else)))))

(fn ConstructionScript
  (|CallParentFunction))

(fn BPIHoldableCallHoldableAction
  (params (Action :type Name :default "None"))
  (switch name Action
    (:Default
      (return false))
    (:StartPrimary
      (CallFunction|ExecEat)
      (return true))))