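; Loot container component that fills itself with random items from the item data table on the server and lets players loot them.
; Players registered as spectators get the contents as an array via a client RPC that opens the lootbox UI.
; Loot requests are validated on authority, move items into the requester's inventory component, then multicast updates to local inventory widgets.
; On EndPlay, non-dedicated instances close the local player's lootbox.
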(event Custom|MULTICAST%20Update
  (params (Added%20Item%20ID :type Name) (Added%20Item%20Data :type S%20Inventory%20System%20Item%20Data%20Structure) (Item%20Added :type Boolean))
  (bind _returnvalue (Game|GetPlayerController 0))
  (if (Utilities|Array|ContainsItem (Variables|Default|GetSpectators) _returnvalue)
    _
    (else
      _))
  (bind _inventory_widget (Class|BPISimpleInventorySystem|BPISimpleInventorySystemGetInventoryWidgetReference(Message) _returnvalue))
  (Utilities|IsValid _inventory_widget
    (:Is%20Valid
      (Class|BPISimpleInventorySystem|BPISimpleInventorySystemonLootboxItemUpdated(Message) _inventory_widget Added%20Item%20ID Added%20Item%20Data Item%20Added self))))

(event Custom|SERVER%20Request%20Loot
  (params (Item%20ID :type Name) (Executing%20Spectator :type Player%20Controller%20Object%20Reference))
  (CallFunction|RequestLoot Item%20ID Executing%20Spectator))

(event EventBeginPlay
  (Networking|SwitchHasAuthority
    (:Authority
      (Networking|SetReplicates (Components|GetOwner) true)
      (CallFunction|GenerateRandomItems))))

(event EventBPISimpleInventorySystemRequestSpectatorRemoval
  (params (To%20Lootbox :type BPC%20SMSK%20Loot%20Component%20Object%20Reference) (Removed%20Spectator :type Player%20Controller%20Object%20Reference))
  (CallFunction|RemoveSpectator Removed%20Spectator))

(event EventEndPlay
  (params (EndPlayReason :type EEndPlayReason%20Enum :default "Destroyed"))
  (|CallParentFunction EndPlayReason)
  (if (not (Networking|IsDedicatedServer))
    (bind _inventory_comp_reference (Class|BPISimpleInventorySystem|BPISimpleInventorySystemGetInventoryComponent(Message) (Game|GetPlayerController 0)))
    (Utilities|IsValid _inventory_comp_reference
      (:Is%20Valid
        (Default|CLIENTCloseLootbox _inventory_comp_reference)))))

(fn OnRepItems)

(fn RequestLoot
  (params (Item%20ID :type Name) (Executing%20Spectator :type Player%20Controller%20Object%20Reference))
  (bind _items (Variables|Default|GetItems))
  (bind (_value _returnvalue) (Utilities|Map|Find _items Item%20ID))
  (Networking|SwitchHasAuthority
    (:Authority
      (Utilities|FlowControl|Sequence
        (:then_0
          (if (Utilities|Array|ContainsItem (Variables|Default|GetSpectators) Executing%20Spectator)
            (if _returnvalue
              (bind _inventory_comp_reference (Class|BPISimpleInventorySystem|BPISimpleInventorySystemGetInventoryComponent(Message) Executing%20Spectator))
              (bind _success (Default|AddItem _inventory_comp_reference Item%20ID _value))
              (if _success
                (CallFunction|MULTICASTUpdate Item%20ID (Utilities|Struct|MakeS_InventorySystem_ItemData 0 0) false)
                (Utilities|Map|Remove (Variables|Default|GetItems) Item%20ID)))))
        (:then_1
          (return))))
    (:Remote
      (return))))

(fn AddSpectator
  (params (New%20Spectator :type Player%20Controller%20Object%20Reference))
  (Utilities|FlowControl|Sequence
    (:then_0
      (if (not (Utilities|Array|ContainsItem (Variables|Default|GetSpectators) New%20Spectator))
        (Utilities|Array|Add (Variables|Default|GetSpectators) New%20Spectator)
        (bind _inventory_comp_reference (Class|BPISimpleInventorySystem|BPISimpleInventorySystemGetInventoryComponent(Message) New%20Spectator))
        (Utilities|IsValid _inventory_comp_reference
          (:Is%20Valid
            (bind _constructred_inventorz (CallFunction|ConstructInventoryforSpectator))
            (Default|CLIENTOpenLootBox _inventory_comp_reference _constructred_inventorz self)))))
    (:then_1
      (return))))

(fn UpdatetoAllSpectators)

(fn ConstructInventoryforSpectator
  (bind _items (Variables|Default|GetItems))
  (bind _keys (Utilities|Map|Keys _items))
  (bind _values (Utilities|Map|Values _items))
  (for (_array_element _array_index) _keys
    (Utilities|Array|Add (LocalVariables|GetL%20Constructed%20Inventory) (Utilities|Struct|MakeS_InventorySystem_InventoryItem _array_element (Utilities|Array|Get(acopy) _values _array_index))))
  (return (LocalVariables|GetL%20Constructed%20Inventory)))

(fn RemoveSpectator
  (params (Removed%20Spectator :type Player%20Controller%20Object%20Reference%20%28by%20ref%29))
  (Utilities|Array|RemoveItem (Variables|Default|GetSpectators) Removed%20Spectator)
  (return))

(fn GenerateRandomItems
  ;[1 1 1] Random Loot spawn
  (bind _outrownames (DataTable|GetDataTableRowNames "/Game/Dreamrise_SMSK/Other/Data/DT_SimpleInventorySystem_ItemData.DT_SimpleInventorySystem_ItemData"))
  (for _index (range 0 (Variables|Default|GetMax%20Loot%20Items))
    (bind _output_get (LocalVariables|SetL%20Item (Utilities|Array|Get(acopy) _outrownames (Math|Random|RandomIntegerinRange 0 (Utilities|Array|LastIndex _outrownames)))))
    (bind _returnvalue (Utilities|GetDataTableRow "/Game/Dreamrise_SMSK/Other/Data/DT_SimpleInventorySystem_ItemData.DT_SimpleInventorySystem_ItemData" _output_get)
      (:then
        (Utilities|Map|Add (Variables|Default|GetItems) (LocalVariables|GetL%20Item) (Utilities|Struct|MakeS_InventorySystem_ItemData (Math|Random|RandomIntegerinRange 1 (Utilities|Struct|BreakS_InventorySystem_FullItemData _returnvalue)) 0))))))

(fn BPISimpleInventorySystemGetInventoryComponent
  (return 0))

(fn BPISimpleInventorySystemGetInventoryWidgetReference
  (return 0))