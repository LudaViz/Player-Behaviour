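; Holdable melee weapon whose primary action starts a rate-limited swing, alternating two montages, with camera shake.
; The swing plays locally at once and replicates through a server-to-multicast RPC that skips the local instance.
; After a retriggerable delay, a camera-aimed sphere trace drives local impact effects.
; A wider body-forward trace supplies effects for remote instances or local aim misses, and applies damage once per actor on authority only.
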(event Custom|Exec%20Attack
  (Utilities|FlowControl|DoOnce false :!label _label
    (:Completed
      (Utilities|FlowControl|Sequence
        (:then_0
          (bind _isa (Utilities|FlowControl|FlipFlop)
            (:A
              _)
            (:B
              _))
          (CallFunction|LocalAttack _isa)
          (CallFunction|SERVERAttack _isa)
          (Utilities|FlowControl|Delay 0.3)
          (Game|Feedback|ClientStartCameraShake (Game|GetPlayerController 0) "/Game/Dreamrise_SMSK/Other/Camera/CMS_Attack.CMS_Attack_C" 2.0 "CameraLocal" "0, 0, 0"))
        (:then_1
          (Utilities|FlowControl|Delay 0.5)
          (goto _label Reset))))))

(event Custom|Multicast%20Attack
  (params (FlipFlop :type Boolean))
  (if (not (CallFunction|IsLocal))
    (CallFunction|LocalAttack FlipFlop)))

(event Custom|SERVER%20Attack
  (params (FlipFlop :type Boolean))
  (CallFunction|MulticastAttack FlipFlop))

(event Custom|Local%20Attack
  (params (Index :type Boolean))
  (bind _ascharacter (Utilities|Casting|CastToCharacter (Game|GetInstigator)))
  (Animation|PlayAnimMontage _ascharacter (select Index "/Game/Dreamrise_SMSK/Animations/A_MeleeAttack_04_Montage.A_MeleeAttack_04_Montage" "/Game/Dreamrise_SMSK/Animations/A_MeleeAttack_03_Montage.A_MeleeAttack_03_Montage") 0.9 "None")
  (Utilities|FlowControl|RetriggerableDelay 0.3)
  (CallFunction|ApplyDamage))

(event EventBeginPlay
  (|CallParentFunction) ; This node is disabled and will not be called.\nDrag off pins to build functionality.
)

(event Collision|EventActorBeginOverlap
  (params (OtherActor :type Actor%20Object%20Reference)))

(event EventTick
  (params (DeltaSeconds :type Float%20%28single-precision%29)))

(fn ConstructionScript
  (|CallParentFunction))

(fn BPIHoldableCallHoldableAction
  (params (Action :type Name :default "None"))
  (switch name Action
    (:Default
      (return false))
    (:StartPrimary
      (CallFunction|ExecAttack)
      (return true))))

(fn ApplyDamage
  (bind _returnvalue (Game|GetInstigator))
  (bind _returnvalue_2 (Game|GetInstigator))
  (bind _returnvalue_3 (Math|Float|MakeLiteralFloat 1.4e+02))
  (bind _returnvalue_4 (Transformation|GetActorLocation _returnvalue_2))
  (bind _returnvalue_5 (Transformation|GetActorLocation _returnvalue))
  (bind _returnvalue_6 (+ _returnvalue_5 "0.000000,0.000000,70.000000"))
  (bind _returnvalue_7 (+ _returnvalue_4 "0.000000,0.000000,30.000000"))
  (Utilities|FlowControl|Sequence
    (:then_0
      (if (CallFunction|IsLocal)
        (bind _outhits (Collision|MultiSphereTraceByChannel _returnvalue_6 (+ _returnvalue_6 (* (Math|Vector|GetForwardVector (Camera|GetCameraRotation (Game|GetPlayerCameraManager 0))) _returnvalue_3)) 4e+01 "TraceTypeQuery1" false (Utilities|Array|MakeArray (Game|GetInstigator)) "None"))
        (for _array_element _outhits
          (if (not (Utilities|Set|Contains (LocalVariables|GetL%20Hit%20Actors) (.HitActor (Collision|BreakHitResult _array_element))))
            (Utilities|Set|Add (LocalVariables|GetL%20Hit%20Actors) (.HitActor (Collision|BreakHitResult _array_element)))
            (Effects|SpawnEmitteratLocation "/Game/Dreamrise_SMSK/Assets/FX/P_ImpactStuff.P_ImpactStuff" (.ImpactPoint (Collision|BreakHitResult _array_element)) "0, 0, 0" "1.000000,1.000000,1.000000" true "AutoRelease")
            (Audio|SpawnSoundatLocation "/Game/Dreamrise_SMSK/Audio/CUE_Impact.CUE_Impact" (.ImpactPoint (Collision|BreakHitResult _array_element)) "0, 0, 0" 1.0 1.0 0.0 "/Game/Dreamrise_SMSK/Audio/Attenuation/SAT_Hit.SAT_Hit" 0)
            (LocalVariables|SetL%20Local%20Hit true)))))
    (:then_1
      (Utilities|Set|Clear (LocalVariables|GetL%20Hit%20Actors))
      (bind _outhits_2 (Collision|MultiSphereTraceByChannel _returnvalue_7 (+ _returnvalue_7 (* (Transformation|GetActorForwardVector _returnvalue_2) _returnvalue_3)) 6e+01 "TraceTypeQuery1" false (Utilities|Array|MakeArray (Game|GetInstigator)) "None"))
      (for _array_element_2 _outhits_2
        (if (not (Utilities|Set|Contains (LocalVariables|GetL%20Hit%20Actors) (.HitActor (Collision|BreakHitResult _array_element_2))))
          (Utilities|Set|Add (LocalVariables|GetL%20Hit%20Actors) (.HitActor (Collision|BreakHitResult _array_element_2)))
          (Utilities|FlowControl|Sequence
            (:then_0
              (if (CallFunction|IsLocal)
                (if (not (LocalVariables|GetL%20Local%20Hit))
                  (Effects|SpawnEmitteratLocation "/Game/Dreamrise_SMSK/Assets/FX/P_ImpactStuff.P_ImpactStuff" (.ImpactPoint (Collision|BreakHitResult _array_element_2)) "0, 0, 0" "1.000000,1.000000,1.000000" true "AutoRelease" :!label _label)
                  (Audio|SpawnSoundatLocation "/Game/Dreamrise_SMSK/Audio/CUE_Impact.CUE_Impact" (.ImpactPoint (Collision|BreakHitResult _array_element_2)) "0, 0, 0" 1.0 1.0 0.0 "/Game/Dreamrise_SMSK/Audio/Attenuation/SAT_Hit.SAT_Hit" 0))
                (else
                  (goto _label))))
            (:then_1
              (Networking|SwitchHasAuthority
                (:Authority
                  (Game|Damage|ApplyDamage (.HitActor (Collision|BreakHitResult _array_element_2)) 2e+01 (Game|GetInstigatorController) self))))))))))