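; Base Blueprint for a beeping proximity detector that scans around the player for targets while active.
; A looping timer runs capsule traces, keeping actors that implement I_TargetForDetectors and lie within a cone ahead of the player.
; The closest target's distance maps to a delay and sound pitch, which StopScan resets.
; Child Blueprints override the empty EffectDetector, called on start and stop; SoundActivate plays the sound at the computed pitch.
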(event Custom|StartScan
  ;[0.007812 0.008203 0.01562] Main logic for target search
  (Variables|Logic|SetActive true)
  (bind _returnvalue (Utilities|Time|SetTimerbyEvent (delegate Custom|Searching) 0.1 true))
  (Variables|Logic|SetScanTimer _returnvalue)
  (CallFunction|SearchTargets)
  (CallFunction|EffectDetector))

(event Custom|Searching
  ;[0.007812 0.008203 0.01562] Main logic for target search
  (CallFunction|SearchTargets)
  (CallFunction|FindClosestTarget (Variables|Logic|GetTargets))
  (CallFunction|ConvertDistance (Variables|Logic|GetClosestTarget)))

(event Custom|StopScan
  ;[0.007812 0.008203 0.01562] Stop detector
  (Variables|Logic|SetActive false)
  (Utilities|Time|ClearandInvalidateTimerbyHandle (Variables|Logic|GetScanTimer))
  (CallFunction|Reset)
  (CallFunction|EffectDetector))

(event EventBeginPlay
  (CallFunction|References))

(fn ConstructionScript
  (Audio|Components|Audio|SetSound (Variables|Default|GetSound) (Variables|BaseOptions|GetTargetSound)))

(fn SearchTargets
  (bind _playercharacter (Variables|References|GetPlayerCharacter))
  (bind _playercharacter_2 (Variables|References|GetPlayerCharacter))
  (bind _returnvalue (Transformation|GetActorLocation _playercharacter))
  (bind _returnvalue_2 (Transformation|GetActorTransform _playercharacter_2))
  ;[0.007812 0.008203 0.01562] Find relevant target for detector
  (bind _outhits (Class|KismetSystemLibrary|CapsuleTraceMultiforObjects _returnvalue _returnvalue (Variables|Baseoptions|GetDetectorRaduis) 0.0 (Variables|BaseOptions|GetTarget%20Type) false 0 "None" true "(R=1.000000,G=0.000000,B=0.000000,A=1.000000)" "(R=0.000000,G=1.000000,B=0.000000,A=1.000000)" 1.0))
  (for _array_element _outhits
    (if (Utilities|DoesObjectImplementInterface (.HitActor (Collision|BreakHitResult _array_element)) "/Game/TrackDecay/Scanner/DetectorBeep/Blueprints/Interfaces/I_TargetForDetectors.I_TargetForDetectors_C")
      (bind _targetfordetector (Class|ITargetforDetectors|TargetforDetectors(Message) (.HitActor (Collision|BreakHitResult _array_element))))
      (if (<= (Class|KismetMathLibrary|DegAcos (Math|Vector|DotProduct (Math|Vector|Normalize (.location (Math|Transform|MakeRelativeTransform (Math|Conversions|ToTransform(Vector) (Transformation|GetActorLocation _targetfordetector)) (Math|Transform|MakeTransform (.location _returnvalue_2) (.rotation _returnvalue_2) "1.000000,1.000000,1.000000")))) "1.000000, 0, 0")) (* (Variables|BaseOptions|GetDetectorAngle) 0.5))
        (Utilities|Array|AddUnique (LocalVariables|GetLocalTargets) _targetfordetector)
        (if (not (Utilities|Array|ContainsItem (Variables|Logic|GetTargets) _targetfordetector))
          (Utilities|Array|AddUnique (Variables|Logic|GetTargets) _targetfordetector)))))
  (for _array_element_2 (Variables|Logic|GetTargets)
    (if (not (Utilities|Array|ContainsItem (LocalVariables|GetLocalTargets) _array_element_2))
      (Utilities|Array|RemoveItem (Variables|Logic|GetTargets) _array_element_2))))

(fn References
  (Variables|References|SetPlayerCharacter (Game|GetPlayerCharacter 0)))

(fn EffectDetector
  ;[0.007812 0.008203 0.01562] This function should be override in child blueprints
)

(fn FindClosestTarget
  (params (Targets :type Array%20of%20Actor%20Object%20References))
  ;[0.007812 0.008203 0.01562] Find closest target
  (if (Utilities|Array|IsNotEmpty Targets)
    (Variables|Logic|SetClosestRange (Transformation|GetDistanceTo (Utilities|Array|Get(acopy) Targets) (Variables|References|GetPlayerCharacter)))
    (for _array_element Targets
      (if (<= (Transformation|GetDistanceTo _array_element (Variables|References|GetPlayerCharacter)) (Variables|Logic|GetClosestRange))
        (Variables|Logic|SetClosestRange (Transformation|GetDistanceTo _array_element (Variables|References|GetPlayerCharacter)))
        (Variables|Logic|SetClosestTarget _array_element)))
    (else
      (Variables|Logic|SetClosestTarget 0))))

(fn ConvertDistance
  (params (ClosestTarget :type Actor%20Object%20Reference))
  (bind _playercharacter (Variables|References|GetPlayerCharacter))
  (bind _returnvalue (Transformation|GetDistanceTo ClosestTarget _playercharacter))
  ;[0.007812 0.008203 0.01562] Convert distance to delay between tick detector and pitching sound
  (Utilities|IsValid ClosestTarget
    (:Is%20Valid
      (Variables|Logic|SetDelay (Math|Float|MapRangeClamped _returnvalue (Variables|Baseoptions|GetDetectorRaduis) 0.0 (Variables|BaseOptions|GetStartDelay) 0.1))
      (Variables|Logic|SetPitch (Math|Float|MapRangeClamped _returnvalue (Variables|Baseoptions|GetDetectorRaduis) 0.0 (Variables|BaseOptions|GetStartPitch) 2.0)))))

(fn Reset
  ;[0.007812 0.008203 0.01562] Set default settings of detector
  (Variables|Logic|SetDelay 1.0)
  (Variables|Logic|SetPitch 0.0)
  (Variables|Logic|SetClosestTarget 0)
  (Utilities|Array|Clear (Variables|Logic|GetTargets)))

(fn SoundActivate
  (Audio|Components|Audio|SetPitchMultiplier (Variables|Default|GetSound) (Variables|Logic|GetPitch))
  (Components|Activation|Activate (Variables|Default|GetSound) false))