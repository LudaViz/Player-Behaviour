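; BP_Wounded is a wounded-figure actor that displays a looping animation picked at random.
; The construction script draws from the Animations array and assigns the pick to the mesh's animation data, so the pose is chosen without runtime logic.
; It implements interaction system functions that refuse interaction and give an empty prompt, while TargetForDetectors returns the actor itself.
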(fn ConstructionScript
  (Variables|/Script/Engine.SkeletalMeshComponent|SetAnimationData (Variables|Character|GetMesh) (Utilities|Struct|MakeSingleAnimationPlayData (.OutItem (Utilities|Array|Random (Variables|Default|GetAnimations))) true true 0.0 1.0)))

(fn BPIInteractionSystemCanInteract
  (return false))

(fn BPIInteractionSystemGetCurrentLocalInteractionActor
  (return 0))

(fn BPIInteractionSystemGetPrompt
  (return ""))

(fn TargetforDetectors
  (return self))