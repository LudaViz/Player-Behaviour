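; BP_WanderingWounded is a pawn, by its name a wounded character, that roams around a Boundary component at random.
; On BeginPlay it picks a navigable point around the Boundary's location, using the box's X extent as radius, and walks there with AI MoveTo.
; On success it pauses for a random few seconds and picks a new point; on failure it retries the same destination after a short delay.
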(event EventBeginPlay
  (bind _boundary (Variables|Default|GetBoundary))
  (bind _returnvalue (Transformation|GetWorldLocation _boundary))
  (bind _randomlocation (Class|NavigationSystemV1|GetRandomLocationinNavigableRadius (Math|Vector|MakeVector (.x _returnvalue) (.y _returnvalue) 0.0) (.x (Variables|/Script/Engine.BoxComponent|GetBoxExtent _boundary)) 0 0 :!label _label))
  (Variables|Default|SetRandom%20Location _randomlocation)
  (AI|AIMoveTo self (Variables|Default|GetRandom%20Location) 0 5e+01 false :!label _label_2
    (:OnSuccess
      (Utilities|FlowControl|RetriggerableDelay (Math|Random|RandomFloatinRange 1.0 5.0))
      (goto _label))
    (:OnFail
      (Utilities|FlowControl|RetriggerableDelay 0.2)
      (goto _label_2))))

(event Collision|EventActorBeginOverlap
  (params (OtherActor :type Actor%20Object%20Reference)))

(event EventTick
  (params (DeltaSeconds :type Float%20%28single-precision%29)))

(fn ConstructionScript)