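; Player inventory component on the PlayerController, storing items by ID with count and ammo, plus primary, secondary and melee weapon slots.
; The server handles adding, removing, dropping and using items, while client events update local data, UI and lootbox screens.
; Equipping a weapon drops the old one, and using items toggles a spawned BP_Holdable.
; Drops spawn BP_LootItem actors, merging non-weapon items into matching nearby pickups via sphere trace.
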(event Custom|SERVER%20Request%20Use%20Item
  (params (Item%20ID :type Name))
  (CallFunction|UseItem Item%20ID))

(event Custom|CLIENT%20On%20Item%20Updated
  (params (Added%20Item%20ID :type Name) (Added%20Item%20Data :type S%20Inventory%20System%20Item%20Data%20Structure) (Item%20Added :type Boolean))
  (bind _inventory (Variables|Default|GetInventory))
  (bind (_item_exists _item_full_data) (CallFunction|GetItemDatafromItemID Added%20Item%20ID))
  (if _item_exists
    (if Item%20Added
      (Utilities|Map|Add _inventory Added%20Item%20ID Added%20Item%20Data)
      (else
        (Utilities|Map|Remove _inventory Added%20Item%20ID)))
    (Default|CallOnItemUpdatedLocal)
    (Audio|PlaySound2D "/Game/Dreamrise_SMSK/Audio/CUE_Backpack.CUE_Backpack" 1.0 1.0 0.0 0 0)
    (if (Math|Boolean|ANDBoolean (Utilities|Enum|NotEqual(Enum) (.ItemType (Utilities|Struct|BreakS_InventorySystem_FullItemData _item_full_data)) "NewEnumerator0") (Utilities|Enum|NotEqual(Enum) (.ItemType (Utilities|Struct|BreakS_InventorySystem_FullItemData _item_full_data)) "NewEnumerator1") (Utilities|Enum|NotEqual(Enum) (.ItemType (Utilities|Struct|BreakS_InventorySystem_FullItemData _item_full_data)) "NewEnumerator2"))
      (bind _inventory_widget (Class|BPISimpleInventorySystem|BPISimpleInventorySystemGetInventoryWidgetReference(Message) (Components|GetOwner)))
      (Utilities|IsValid _inventory_widget
        (:Is%20Valid
          (Class|BPISimpleInventorySystem|BPISimpleInventorySystemonItemUpdated(Message) _inventory_widget Added%20Item%20ID Added%20Item%20Data Item%20Added))))))

(event Custom|Bind%20Holdable%20On%20Destroyed%20Event
  (Game|BindEventtoOnDestroyed (Variables|Default|GetHoldable%20Reference) (delegate Custom|On%20Holdable%20Destroyed)))

(event Custom|SERVER%20Request%20Drop
  (params (Item%20ID :type Name) (Amount :type Integer))
  (CallFunction|DropItem Item%20ID Amount))

(event Custom|CLIENT%20Update%20Weapon%20ID
  (params (New%20Weapon%20ID :type Name) (Item%20Type :type E_InventorySystem_ItemType%20Enum :default "NewEnumerator0"))
  ;[1 1 1] Update Weapon ID to client, send to proper widgets to update them
  (Audio|PlaySound2D "/Game/Dreamrise_SMSK/Audio/CUE_Backpack.CUE_Backpack" 1.0 1.0 0.0 0 0)
  (Utilities|FlowControl|Sequence
    (:then_0
      (switch Utilities|FlowControl|Switch|SwitchonE_InventorySystem_ItemType Item%20Type
        (:NewEnumerator0
          (Variables|Default|SetPrimary%20Weapon%20ID New%20Weapon%20ID))
        (:NewEnumerator1
          (Variables|Default|SetSecondary%20Weapon%20ID New%20Weapon%20ID))
        (:NewEnumerator2
          (Variables|Default|SetMelee%20Weapon%20ID New%20Weapon%20ID))))
    (:then_1
      (bind _inventory_widget (Class|BPISimpleInventorySystem|BPISimpleInventorySystemGetInventoryWidgetReference(Message) (Components|GetOwner)))
      (Utilities|IsValid _inventory_widget
        (:Is%20Valid
          (Class|BPISimpleInventorySystem|BPISimpleInventorySystemonWeaponIDUpdated(Message) _inventory_widget New%20Weapon%20ID Item%20Type))))
    (:then_2
      (bind _main_ui (Class|BPIPlayerBase|BPIPlayerBaseGetMainUI(Message) (Components|GetOwner)))
      (Utilities|IsValid _main_ui
        (:Is%20Valid
          (Class|BPISimpleInventorySystem|BPISimpleInventorySystemonWeaponIDUpdated(Message) _main_ui New%20Weapon%20ID Item%20Type))))))

(event Custom|On%20Holdable%20Destroyed
  (params (DestroyedActor :type Actor%20Object%20Reference))
  (EventDispatchers|UnbindallEventsfromOnDestroyed (Variables|Default|GetHoldable%20Reference))
  (Variables|Default|SetHoldable%20ID "None")
  (Variables|Default|SetHoldable%20Reference 0)
  (Class|BPISimpleInventorySystem|BPISimpleInventorySystemSetHoldable(Message) (Components|GetOwner))
  (CallFunction|CLIENTUpdateHoldable (Variables|Default|GetHoldable%20ID)))

(event Custom|CLIENT%20Update%20Holdable
  (params (New%20Holdable%20ID :type Name))
  (Variables|Default|SetHoldable%20ID New%20Holdable%20ID)
  (Audio|PlaySound2D "/Game/Dreamrise_SMSK/Audio/CUE_Backpack.CUE_Backpack" 1.0 1.0 0.0 0 0)
  (bind _main_ui (Class|BPIPlayerBase|BPIPlayerBaseGetMainUI(Message) (Components|GetOwner)))
  (Utilities|IsValid _main_ui
    (:Is%20Valid
      (Class|BPISimpleInventorySystem|BPISimpleInventorySystemonHoldableUpdated(Message) _main_ui (Variables|Default|GetHoldable%20ID)))))

(event Custom|CLIENT%20Open%20LootBox
  (params (Items :type Array%20of%20S%20Inventory%20System%20Inventory%20Item%20Structures) (Lootbox%20Reference :type BPC%20SMSK%20Loot%20Component%20Object%20Reference%20%28by%20ref%29))
  (bind _main_ui (Class|BPIPlayerBase|BPIPlayerBaseGetMainUI(Message) (Components|GetOwner)))
  (Utilities|IsValid _main_ui
    (:Is%20Valid
      (Class|BPIPlayerUserInterface|BPIPlayerUserInterfaceOpenLootbox(Message) _main_ui Items Lootbox%20Reference))))

(event Custom|CLIENT%20Close%20Lootbox
  (bind _main_ui (Class|BPIPlayerBase|BPIPlayerBaseGetMainUI(Message) (Components|GetOwner)))
  (Utilities|IsValid _main_ui
    (:Is%20Valid
      (Class|BPIPlayerUserInterface|BPIPlayerUserInterfaceCloseLootbox(Message) _main_ui))))

(event EventEndPlay
  (params (EndPlayReason :type EEndPlayReason%20Enum :default "Destroyed"))
  ;[1 1 1] Make sure we destroy holdable when disconnected
  (|CallParentFunction EndPlayReason)
  (bind _holdable_reference (Variables|Default|GetHoldable%20Reference)
    (:then
      (Actor|DestroyActor _holdable_reference))
    (:else)))

(fn AddItem
  (params (Item%20ID :type Name) (Item%20Data :type S%20Inventory%20System%20Item%20Data%20Structure))
  (bind _inventory (Variables|Default|GetInventory))
  (bind (_value _returnvalue) (Utilities|Map|Find _inventory Item%20ID))
  (Networking|SwitchHasAuthority
    (:Authority
      (bind (_item_exists _item_full_data) (CallFunction|GetItemDatafromItemID Item%20ID))
      (if _item_exists
        (if (> (.ItemCount (Utilities|Struct|BreakS_InventorySystem_ItemData Item%20Data)) 0)
          (Utilities|FlowControl|Sequence ; After return failed (not executed)
            (:then_0
              ;[1 1 1] Update Weapon ID if Item is a weapon (Melee, Secondary, Primary), otherwise continue with sequence to add it into inventory
              ; Drop old Weapon when ID is valid
              (switch Utilities|FlowControl|Switch|SwitchonE_InventorySystem_ItemType (.ItemType (Utilities|Struct|BreakS_InventorySystem_FullItemData _item_full_data))
                (:NewEnumerator0
                  (if (== (Variables|Default|GetPrimary%20Weapon%20ID) "")
                    _
                    (else
                      (CallFunction|DropItem (Variables|Default|GetPrimary%20Weapon%20ID) 1)))
                  (bind _output_get (Variables|Default|SetPrimary%20Weapon%20ID Item%20ID))
                  (CallFunction|CLIENTUpdateWeaponID _output_get "NewEnumerator0"))
                (:NewEnumerator1
                  (if (== (Variables|Default|GetSecondary%20Weapon%20ID) "")
                    _
                    (else
                      (CallFunction|DropItem (Variables|Default|GetSecondary%20Weapon%20ID) 1)))
                  (bind _output_get_2 (Variables|Default|SetSecondary%20Weapon%20ID Item%20ID))
                  (CallFunction|CLIENTUpdateWeaponID _output_get_2 "NewEnumerator1"))
                (:NewEnumerator2
                  (if (== (Variables|Default|GetMelee%20Weapon%20ID) "")
                    _
                    (else
                      (CallFunction|DropItem (Variables|Default|GetMelee%20Weapon%20ID) 1)))
                  (bind _output_get_3 (Variables|Default|SetMelee%20Weapon%20ID Item%20ID))
                  (CallFunction|CLIENTUpdateWeaponID _output_get_3 "NewEnumerator2")))
              ;[1 1 1] Add Item for data without showing it
              (Utilities|Map|Add (Variables|Default|GetInventory) Item%20ID (Utilities|Struct|MakeS_InventorySystem_ItemData 1 (Utilities|Struct|BreakS_InventorySystem_ItemData Item%20Data)))
              (return true) ; MUST BE HERE IN ORDER NOT TO CONTINUE!
            )
            (:then_1
              ;[1 1 1] Already Contains Item
              (if _returnvalue
                (bind _structout (Utilities|Struct|SetmembersinS_InventorySystem_ItemData _value (+ (.ItemCount (Utilities|Struct|BreakS_InventorySystem_ItemData _value)) (Utilities|Struct|BreakS_InventorySystem_ItemData Item%20Data))))
                (Utilities|Map|Add (Variables|Default|GetInventory) Item%20ID _structout)
                (else
                  (Utilities|Map|Add (Variables|Default|GetInventory) Item%20ID Item%20Data)))
              (CallFunction|CLIENTonItemUpdated Item%20ID (.Value (Utilities|Map|Find (Variables|Default|GetInventory) Item%20ID)) true)
              (return true)))
          (else
            _)))
      (return false))))

(fn RemoveItem
  (params (Item%20ID :type Name) (Amount :type Integer))
  (bind _inventory (Variables|Default|GetInventory))
  (bind (_value _returnvalue) (Utilities|Map|Find _inventory Item%20ID))
  (Networking|SwitchHasAuthority
    (:Authority
      (if (> Amount 0)
        (bind (_item_exists _item_full_data) (CallFunction|GetItemDatafromItemID Item%20ID))
        (if _item_exists
          (Utilities|FlowControl|Sequence
            (:then_0
              (if (== (Variables|Default|GetHoldable%20ID) Item%20ID)
                (bind _holdable_reference (Variables|Default|GetHoldable%20Reference)
                  (:then
                    (Actor|DestroyActor _holdable_reference))
                  (:else))))
            (:then_1
              (Utilities|FlowControl|Sequence ; After return failed (not executed)
                (:then_0
                  ;[1 1 1] If Requested Item is a weapon (Primary, Melee, Secondary), try to obtain if player has the weapon, if yes, remove it, update data and continue
                  (switch Utilities|FlowControl|Switch|SwitchonE_InventorySystem_ItemType (.ItemType (Utilities|Struct|BreakS_InventorySystem_FullItemData _item_full_data))
                    (:NewEnumerator0
                      (if (!= (Variables|Default|GetPrimary%20Weapon%20ID) "")
                        (bind _output_get (Variables|Default|SetPrimary%20Weapon%20ID "None"))
                        (CallFunction|CLIENTUpdateWeaponID _output_get "NewEnumerator0")
                        (Utilities|Map|Remove (Variables|Default|GetInventory) Item%20ID :!label _label)
                        (return true 1) ; MUST BE HERE IN ORDER NOT TO CONTINUE!
                        (else
                          _)))
                    (:NewEnumerator1
                      (if (!= (Variables|Default|GetSecondary%20Weapon%20ID) "")
                        (bind _output_get_2 (Variables|Default|SetSecondary%20Weapon%20ID "None"))
                        (CallFunction|CLIENTUpdateWeaponID _output_get_2 "NewEnumerator1")
                        (goto _label)
                        (else
                          _)))
                    (:NewEnumerator2
                      (if (!= (Variables|Default|GetMelee%20Weapon%20ID) "")
                        (bind _output_get_3 (Variables|Default|SetMelee%20Weapon%20ID "None"))
                        (CallFunction|CLIENTUpdateWeaponID _output_get_3 "NewEnumerator2")
                        (goto _label)
                        (else
                          _))))
                  (return false 0) ; MUST BE HERE IN ORDER NOT TO CONTINUE!
                )
                (:then_1
                  ;[1 1 1] Already Contains Item
                  (if _returnvalue
                    (bind _output_get_4 (LocalVariables|SetL%20Cached%20Item%20Sound (.ItemCount (Utilities|Struct|BreakS_InventorySystem_ItemData _value))))
                    (bind _output_get_5 (LocalVariables|SetL%20New%20Amount (- _output_get_4 Amount)))
                    (if (< _output_get_5 0)
                      (Utilities|Map|Remove (Variables|Default|GetInventory) Item%20ID)
                      (CallFunction|CLIENTonItemUpdated :Added%20Item%20ID Item%20ID)
                      (return true (LocalVariables|GetL%20Cached%20Item%20Sound))
                      (else
                        (bind _structout (Utilities|Struct|SetmembersinS_InventorySystem_ItemData _value (LocalVariables|GetL%20New%20Amount)))
                        (Utilities|Map|Add (Variables|Default|GetInventory) Item%20ID _structout)
                        (CallFunction|CLIENTonItemUpdated Item%20ID (.Value (Utilities|Map|Find (Variables|Default|GetInventory) Item%20ID)) true)
                        (return true Amount)))
                    (else
                      (return false 0)))))))
          (else
            (return false 0)))
        (else
          (return false 0))))))

(fn DropItem
  (params (Item%20ID :type Name) (Amount :type Integer))
  (bind _inventory (Variables|Default|GetInventory))
  (bind (_value _returnvalue) (Utilities|Map|Find _inventory Item%20ID))
  (Networking|SwitchHasAuthority
    (:Authority
      ;[1 1 1] Cache Data for Dropped item
      (if _returnvalue
        (LocalVariables|SetL%20Cached%20Data _value)
        ;[1 1 1] Remove Item and determine correct removed amount
        (bind (_success _removed_amount) (CallFunction|RemoveItem Item%20ID Amount))
        (if _success
          (LocalVariables|SetL%20Removed%20Amount _removed_amount)
          (Utilities|FlowControl|Sequence
            (:then_0
              ;[1 1 1] If holdable, Destroyed
              (if (== (Variables|Default|GetHoldable%20ID) Item%20ID)
                (bind _holdable_reference (Variables|Default|GetHoldable%20Reference)
                  (:then
                    (Actor|DestroyActor _holdable_reference))
                  (:else))))
            (:then_1
              (LocalVariables|SetL%20Drop%20Location (+ (Transformation|GetActorLocation (Pawn|GetControlledPawn (.AsPlayer%20Controller (Utilities|Casting|CastToPlayerController (Components|GetOwner))))) (Math|Vector|MakeVector (Math|Random|RandomFloatinRange 2e+01 6e+01) (Math|Random|RandomFloatinRange 2e+01 6e+01) 45.0)))
              (bind _item_full_data (CallFunction|GetItemDatafromItemID Item%20ID))
              (switch Utilities|FlowControl|Switch|SwitchonE_InventorySystem_ItemType (.ItemType (Utilities|Struct|BreakS_InventorySystem_FullItemData _item_full_data))
                (:NewEnumerator0
                  _)
                (:NewEnumerator1
                  _)
                (:NewEnumerator2
                  _)
                (:NewEnumerator3
                  ;[1 1 1] Trace for items with same ID nearby, if found, do not spawn new item, rather add count to item nearby
                  (bind (_outhits _returnvalue_2) (Collision|MultiSphereTraceByChannel (LocalVariables|GetL%20Drop%20Location) (LocalVariables|GetL%20Drop%20Location) 4e+02 "TraceTypeQuery1" false 0 "None"))
                  (if _returnvalue_2
                    (for _array_element _outhits
                      (bind _asbp_loot_item (Utilities|Casting|CastToBP_LootItem (.HitActor (Collision|BreakHitResult _array_element))))
                      (if (== (Variables|/Game/Dreamrise_SMSK/Blueprints/BP_LootItem.BP_LootItem_C|GetItem%20ID _asbp_loot_item) Item%20ID)
                        (bind _structout (Utilities|Struct|SetmembersinS_InventorySystem_ItemData (Variables|/Game/Dreamrise_SMSK/Blueprints/BP_LootItem.BP_LootItem_C|GetItem%20Data _asbp_loot_item) (+ (.ItemCount (Utilities|Struct|BreakS_InventorySystem_ItemData (Variables|/Game/Dreamrise_SMSK/Blueprints/BP_LootItem.BP_LootItem_C|GetItem%20Data _asbp_loot_item))) (LocalVariables|GetL%20Removed%20Amount))))
                        (Variables|/Game/Dreamrise_SMSK/Blueprints/BP_LootItem.BP_LootItem_C|SetItem%20Data _asbp_loot_item _structout)
                        (return))))))
              ;[1 1 1] Keep data except Amount
              (bind _structout_2 (Utilities|Struct|SetmembersinS_InventorySystem_ItemData (LocalVariables|GetL%20Cached%20Data) (LocalVariables|GetL%20Removed%20Amount)))
              ;[1 1 1] Spawn Brand new item in world
              (Game|SpawnActorfromClass "/Game/Dreamrise_SMSK/Blueprints/BP_LootItem.BP_LootItem_C" (Math|Transform|MakeTransform (LocalVariables|GetL%20Drop%20Location) "0, 0, 0" "1.000000,1.000000,1.000000") "AdjustIfPossibleButAlwaysSpawn" "MultiplyWithRoot" 0 Item%20ID _structout_2 true 0)
              (return))))))))

(fn UseItem
  (params (Item%20ID :type Name))
  (Networking|SwitchHasAuthority
    (:Authority
      (bind (_item_exists _item_full_data) (CallFunction|GetItemDatafromItemID Item%20ID))
      (if _item_exists
        (Utilities|FlowControl|Sequence
          (:then_0
            (if (Utilities|IsValidSoftClassReference (.HoldableClass (Utilities|Struct|BreakS_InventorySystem_FullItemData _item_full_data)))
              (LocalVariables|SetL%20Same%20ID%20Cache (!= (Variables|Default|GetHoldable%20ID) Item%20ID))
              (bind _holdable_reference (Variables|Default|GetHoldable%20Reference)
                (:then
                  (Actor|DestroyActor _holdable_reference)
                  (if (not (LocalVariables|GetL%20Same%20ID%20Cache))
                    (return false)))
                (:else))))
          (:then_1
            (Utilities|FlowControl|Sequence
              (:then_0
                (switch Utilities|FlowControl|Switch|SwitchonE_InventorySystem_ItemType (.ItemType (Utilities|Struct|BreakS_InventorySystem_FullItemData _item_full_data))
                  (:NewEnumerator0
                    (if (== (Variables|Default|GetPrimary%20Weapon%20ID) Item%20ID)
                      (bind _returnvalue (Utilities|LoadClassAssetBlocking (.HoldableClass (Utilities|Struct|BreakS_InventorySystem_FullItemData _item_full_data)) :!label _label))
                      (bind _asbp_holdable (Utilities|Casting|CastToBP_HoldableClass _returnvalue))
                      (bind _returnvalue_2 (Game|SpawnActorfromClass _asbp_holdable (Math|Transform|MakeTransform "0, 0, 0" "0, 0, 0" "1.000000,1.000000,1.000000") "AlwaysSpawn" "MultiplyWithRoot" (Components|GetOwner) Item%20ID (Pawn|GetControlledPawn (.AsPlayer%20Controller (Utilities|Casting|CastToPlayerController (Components|GetOwner))))))
                      (Variables|Default|SetHoldable%20Reference _returnvalue_2)
                      (Variables|Default|SetHoldable%20ID Item%20ID)
                      (CallFunction|BindHoldableonDestroyedEvent)
                      (CallFunction|CLIENTUpdateHoldable (Variables|Default|GetHoldable%20ID))
                      (return true)))
                  (:NewEnumerator1
                    (if (== (Variables|Default|GetSecondary%20Weapon%20ID) Item%20ID)
                      (goto _label)))
                  (:NewEnumerator2
                    (if (== (Variables|Default|GetMelee%20Weapon%20ID) Item%20ID)
                      (goto _label)))
                  (:NewEnumerator3
                    (goto _label))))
              (:then_1
                (if (.ReturnValue (Utilities|Map|Find (Variables|Default|GetInventory) Item%20ID))
                  (goto _label))))))
        (else
          (return false))))))

(fn GetItemAmount
  (params (Item%20ID :type Name))
  (bind _inventory (Variables|Default|GetInventory))
  (bind (_value _returnvalue) (Utilities|Map|Find _inventory Item%20ID))
  (if _returnvalue
    (return (Utilities|Struct|BreakS_InventorySystem_ItemData _value))
    (else
      (return 0))))

(fn ModifyItemAmmo
  (params (Item%20ID :type Name%20%28by%20ref%29) (New%20Ammo%20Amount :type Integer) (Update%20Client :type Boolean))
  (bind _inventory (Variables|Default|GetInventory))
  (bind (_value _returnvalue) (Utilities|Map|Find _inventory Item%20ID))
  (Utilities|FlowControl|Sequence
    (:then_0
      (Networking|SwitchHasAuthority
        (:Authority
          ;[1 1 1] Item Exists
          (if _returnvalue
            ;[1 1 1] Modify new Ammo
            (bind _structout (Utilities|Struct|SetmembersinS_InventorySystem_ItemData _value New%20Ammo%20Amount))
            (Utilities|Map|Add (Variables|Default|GetInventory) Item%20ID _structout)
            ;[1 1 1] Wheter update data on client too
            (if Update%20Client
              (CallFunction|CLIENTonItemUpdated Item%20ID (.Value (Utilities|Map|Find (Variables|Default|GetInventory) Item%20ID)) true))))))
    (:then_1
      (return))))

(fn GetItemAmmo
  (params (Item%20ID :type Name))
  (bind _inventory (Variables|Default|GetInventory))
  (bind (_value _returnvalue) (Utilities|Map|Find _inventory Item%20ID))
  (if _returnvalue
    (return (.Ammo (Utilities|Struct|BreakS_InventorySystem_ItemData _value)))
    (else
      (return 0))))