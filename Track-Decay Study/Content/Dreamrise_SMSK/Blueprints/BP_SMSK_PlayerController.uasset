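; Player controller for the SMSK game that hosts the simple inventory component and creates the main UI with a welcome sound for the local player.
; Input toggles the inventory and forwards primary, reload and scroll actions to the held item as named interface messages.
; Server events handle loot requests, lootbox spectator removal and building, where a gate checks recipe amounts before consuming items and spawning a replicated actor.
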(event Custom|SERVER%20Remove%20from%20Lootbox
  (params (To%20Lootbox :type BPC%20SMSK%20Loot%20Component%20Object%20Reference))
  ;[1 1 1] Request remove from Spectating
  (Utilities|IsValid To%20Lootbox
    (:Is%20Valid
      (Class|BPISimpleInventorySystem|BPISimpleInventorySystemRequestSpectatorRemoval(Message) To%20Lootbox 0 self))))

(event Custom|SEVRER%20Request%20Build
  (params (Building%20Class :type BP%20Building%20Base%20Class%20Reference) (Building%20Transform :type Transform) (Recipe :type Array%20of%20S%20Inventory%20System%20Inventory%20Item%20Short%20Structures))
  ;[1 0.1514 0.7386] Request Server to build object
  (Utilities|FlowControl|Sequence
    (:then_0
      (goto _label Open))
    (:then_1
      (for _array_element Recipe
        (bind _amount (Default|GetItemAmount (Variables|Default|GetBPC_SimpleInventorySystem) (.ItemID (Utilities|Struct|BreakS_InventorySystem_InventoryItemShort _array_element))))
        (if (not (>= _amount (.Amount (Utilities|Struct|BreakS_InventorySystem_InventoryItemShort _array_element))))
          (goto _label Close)))
      (Utilities|FlowControl|Gate true :!label _label
        (:Exit
          (for _array_element_2 Recipe
            (Default|RemoveItem (Variables|Default|GetBPC_SimpleInventorySystem) (.itemid _array_element_2) (.amount _array_element_2)))
          (bind _returnvalue (Game|SpawnActorfromClass Building%20Class Building%20Transform "AdjustIfPossibleButAlwaysSpawn" "MultiplyWithRoot" 0 false 5e+02 0))
          (Networking|SetReplicates _returnvalue true))))))

(event Custom|SERVER%20Request%20Add%20Loot
  (params (Loot%20Component :type BPC%20SMSK%20Loot%20Component%20Object%20Reference) (Item%20ID :type Name) (Executing%20Spectator :type Player%20Controller%20Object%20Reference))
  ;[1 1 1] Requets loot from Loot component
  (Default|RequestLoot Loot%20Component Item%20ID Executing%20Spectator))

(event Input|EnhancedActionEvents|EnhancedInputActionIA_ToggleInventory
  (params (ActionValue :type Boolean) (ElapsedSeconds :type Float%20%28double-precision%29) (TriggeredSeconds :type Float%20%28double-precision%29) (InputAction :type Input%20Action%20Object%20Reference :default "/Game/Dreamrise_SMSK/Input/Actions/IA_ToggleInventory.IA_ToggleInventory"))
  (Development|PrintString "Hello")
  (Default|ToggleInventory (Variables|Default|GetUI%20Widget)))

(event Input|EnhancedActionEvents|EnhancedInputActionIA_Reload
  (params (ActionValue :type Boolean) (ElapsedSeconds :type Float%20%28double-precision%29) (TriggeredSeconds :type Float%20%28double-precision%29) (InputAction :type Input%20Action%20Object%20Reference :default "/Game/Dreamrise_SMSK/Input/Actions/IA_Reload.IA_Reload"))
  (bind _holdable_reference (Variables|/Game/Dreamrise_SMSK/Blueprints/Components/BPC_SimpleInventorySystem.BPC_SimpleInventorySystem_C|GetHoldable%20Reference (Variables|Default|GetBPC_SimpleInventorySystem))
    (:then
      (if ActionValue
        (Class|BPIHoldable|BPIHoldableCallHoldableAction(Message) _holdable_reference "Reload")))
    (:else)))

(event Input|EnhancedActionEvents|EnhancedInputActionIA_PrimaryAction
  (params (ActionValue :type Boolean) (ElapsedSeconds :type Float%20%28double-precision%29) (TriggeredSeconds :type Float%20%28double-precision%29) (InputAction :type Input%20Action%20Object%20Reference :default "/Game/Dreamrise_SMSK/Input/Actions/IA_PrimaryAction.IA_PrimaryAction"))
  (bind _holdable_reference (Variables|/Game/Dreamrise_SMSK/Blueprints/Components/BPC_SimpleInventorySystem.BPC_SimpleInventorySystem_C|GetHoldable%20Reference (Variables|Default|GetBPC_SimpleInventorySystem))
    (:then
      (if ActionValue
        (Class|BPIHoldable|BPIHoldableCallHoldableAction(Message) _holdable_reference "StartPrimary")
        (else
          (Class|BPIHoldable|BPIHoldableCallHoldableAction(Message) _holdable_reference "StopPrimary"))))
    (:else)))

(event EventBeginPlay
  ;[1 1 1] On Begin play, create widget and play intro sound
  (if (Pawn|IsLocalController)
    (bind _returnvalue (UserInterface|CreateWidget "/Game/Dreamrise_SMSK/Blueprints/Widgets/W_MainUI.W_MainUI_C" self))
    (bind _output_get (Variables|Default|SetUI%20Widget _returnvalue))
    (UserInterface|Viewport|AddtoViewport _output_get 0)
    (Audio|PlaySound2D "/Game/Dreamrise_SMSK/Audio/CUE_Welcome.CUE_Welcome" 1.0 1.0 0.0 0 0)))

(event EventBPISimpleInventorySystemRequestSpectatorRemoval
  (params (To%20Lootbox :type BPC%20SMSK%20Loot%20Component%20Object%20Reference) (Removed%20Spectator :type Player%20Controller%20Object%20Reference))
  ;[1 1 1] Request remove from Spectating
  (CallFunction|SERVERRemovefromLootbox To%20Lootbox))

(event Input|KeyboardEvents|DebugKeyDelete
  (params (Key :type Key%20Structure :default "None") (ActionValue :type Input%20Action%20Value%20Structure))
  (:Pressed
    (Viewport|RemoveAllWidgets)))

(event Input|MouseEvents|MouseWheelUp
  (params (Key :type Key%20Structure :default "None"))
  (:Pressed
    (bind _holdable_reference (Variables|/Game/Dreamrise_SMSK/Blueprints/Components/BPC_SimpleInventorySystem.BPC_SimpleInventorySystem_C|GetHoldable%20Reference (Variables|Default|GetBPC_SimpleInventorySystem))
      (:then
        (Class|BPIHoldable|BPIHoldableCallHoldableAction(Message) _holdable_reference "ScrollUp"))
      (:else))))

(event Input|MouseEvents|MouseWheelDown
  (params (Key :type Key%20Structure :default "None"))
  (:Pressed
    (bind _holdable_reference (Variables|/Game/Dreamrise_SMSK/Blueprints/Components/BPC_SimpleInventorySystem.BPC_SimpleInventorySystem_C|GetHoldable%20Reference (Variables|Default|GetBPC_SimpleInventorySystem))
      (:then
        (Class|BPIHoldable|BPIHoldableCallHoldableAction(Message) _holdable_reference "ScrollDown"))
      (:else))))

(fn ConstructionScript)

(fn BPIPlayerBaseGetMainUI
  (return (Variables|Default|GetUI%20Widget)))

(fn BPISimpleInventorySystemGetInventoryComponent
  (return (Variables|Default|GetBPC_SimpleInventorySystem)))

(fn BPISimpleInventorySystemGetInventoryWidgetReference
  (bind _ui_widget (Variables|Default|GetUI%20Widget)
    (:then
      (return (Variables|/Game/Dreamrise_SMSK/Blueprints/Widgets/W_MainUI.W_MainUI_C|GetW_InventoryScreen _ui_widget)))
    (:else
      (return 0))))