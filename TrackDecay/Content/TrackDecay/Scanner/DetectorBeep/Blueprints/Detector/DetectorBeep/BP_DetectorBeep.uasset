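; Beeping detector Blueprint that extends a parent detector with a repeating sound and a glowing body material while active.
; EffectDetector starts the Beep timer and raises emissive on a dynamic material built in the Construction Script, or calls ResetDetector to clear both.
; Each tick plays the sound only when Targets is non-empty, then re-arms the looping timer so the interval picks up the current Delay.
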(event Custom|Beep
  ;[0.007812 0.008203 0.01562] Detector effect (Sound)
  (bind _returnvalue (Utilities|Time|SetTimerbyEvent (delegate Custom|ActivateSound) (Variables|Default|GetDelay) true))
  (Variables|Default|SetBeepTimer _returnvalue))

(event Custom|ActivateSound
  ;[0.007812 0.008203 0.01562] Detector effect (Sound)
  (if (not (Utilities|Array|IsEmpty (Variables|Default|GetTargets)))
    (CallFunction|SoundActivate)
    (CallFunction|Beep)))

(event EventBeginPlay
  (|CallParentFunction) ; This node is disabled and will not be called.\nDrag off pins to build functionality.
)

(fn ConstructionScript
  (|CallParentFunction)
  (bind _returnvalue (Rendering|Material|CreateDynamicMaterialInstance (Variables|Default|GetDetectorBody) 1 0 "None" :!class /Script/Engine.PrimitiveComponent))
  (Variables|Default|SetTriggerMat _returnvalue))

(fn EffectDetector
  ;[0.007812 0.008203 0.01562] Start/Stop effect detector
  (|CallParentFunction)
  (if (Variables|Default|GetActive)
    (CallFunction|Beep)
    (Rendering|Material|SetScalarParameterValue (Variables|Default|GetTriggerMat) "Emissive" 5.0 :!class /Script/Engine.MaterialInstanceDynamic)
    (else
      (CallFunction|ResetDetector))))

(fn ResetDetector
  ;[0.007812 0.008203 0.01562] Set default settings of detector
  (Utilities|Time|ClearandInvalidateTimerbyHandle (Variables|Default|GetBeepTimer))
  (Rendering|Material|SetScalarParameterValue (Variables|Default|GetTriggerMat) "Emissive" 0.0 :!class /Script/Engine.MaterialInstanceDynamic))