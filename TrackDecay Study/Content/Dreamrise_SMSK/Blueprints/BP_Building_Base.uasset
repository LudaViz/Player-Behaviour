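; BP_Building_Base is a base building actor that serves as either a placement ghost or a solid, damageable building.
; On BeginPlay, the IsGhost flag either applies the ghost material and disables mesh collision, or enables collision and turns on replication.
; Any damage subtracts from Health, and the actor destroys itself once Health reaches zero or below.
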(event Game|Damage|EventAnyDamage
  (params (Damage :type Float%20%28single-precision%29) (DamageType :type Damage%20Type%20Object%20Reference) (InstigatedBy :type Controller%20Object%20Reference) (DamageCauser :type Actor%20Object%20Reference))
  ;[1 1 1] Apply Damage, remove health, if health is 0 destroy Building
  (bind _output_get (Variables|Default|SetHealth (- (Variables|Default|GetHealth) Damage)))
  (if (<= _output_get 0.0)
    (Actor|DestroyActor)))

(event EventBeginPlay
  ;[1 0.1266 0.1545] Begin Play, determine if it is building ghost, if yes = apply ghost material and no collision, if not = replicate and set collision enabled
  (|CallParentFunction)
  (if (Variables|Default|GetbIsGhost)
    (Rendering|Material|SetMaterial (Variables|Default|GetStaticMesh) 0 "/Game/Dreamrise_SMSK/Assets/Materials/M_BuildingGhost.M_BuildingGhost")
    (Collision|SetCollisionEnabled (Variables|Default|GetStaticMesh) "NoCollision")
    (else
      (Collision|SetCollisionEnabled (Variables|Default|GetStaticMesh) "QueryAndPhysics")
      (Networking|SetReplicates true))))

(fn ConstructionScript)