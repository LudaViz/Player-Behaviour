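; BP_Harvestable is a world actor that players damage to harvest an item into their inventory.
; AnyDamage lowers Health; at zero, with a valid instigator, it fetches the inventory component from that controller via the Simple Inventory System interface.
; It adds ItemToGive only if the controlled pawn is nearby, then destroys itself regardless and flushes net dormancy.
; The construction script gives it a random uniform scale.
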(event Game|Damage|EventAnyDamage
  (params (Damage :type Float%20%28single-precision%29) (DamageType :type Damage%20Type%20Object%20Reference) (InstigatedBy :type Controller%20Object%20Reference) (DamageCauser :type Actor%20Object%20Reference))
  (bind _returnvalue (Pawn|GetControlledPawn InstigatedBy))
  (bind _output_get (Variables|Default|SetHealth (- (Variables|Default|GetHealth) Damage)))
  (if (<= _output_get 0.0)
    (Utilities|IsValid InstigatedBy
      (:Is%20Valid
        (Utilities|FlowControl|Sequence
          (:then_0
            (bind _inventory_comp_reference (Class|BPISimpleInventorySystem|BPISimpleInventorySystemGetInventoryComponent(Message) InstigatedBy))
            (Utilities|IsValid _inventory_comp_reference
              (:Is%20Valid
                (Utilities|IsValid _returnvalue
                  (:Is%20Valid
                    (if (< (Transformation|GetDistanceTo _returnvalue) 5e+02)
                      (Default|AddItem _inventory_comp_reference (Variables|Default|GetItem%20to%20Give) (Utilities|Struct|MakeS_InventorySystem_ItemData (Variables|Default|GetAmount%20to%20Give) 0))))))))
          (:then_1
            (Actor|DestroyActor)
            (Networking|FlushNetDormancy)
            (Networking|ForceNetUpdate)))))))

(fn ConstructionScript
  (Transformation|SetActorScale3D (Math|Conversions|ToVector(Float) (Math|Random|RandomFloatinRange 1.0 2.0))))