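; BP_WoundedSpawner spawns wandering wounded AI humans on request through its SpawnHuman event.
; After a random delay of a few seconds, it spawns the pawn high above its own location.
; It casts the pawn to BP_Wounded, then hands it the spawner's Box as Boundary and the requested PlayerColor.
; The GetRandomFloatFromBoxExtent helper feeds the X/Y offsets, but its random-range calculation is left unused.
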(event Custom|SpawnHuman
  (params (PlayerColor :type Linear%20Color%20Structure))
  (bind _box (Variables|Default|GetBox))
  (bind _boxextent (Variables|/Script/Engine.BoxComponent|GetBoxExtent _box))
  (Utilities|FlowControl|Delay (Math|Random|RandomFloatinRange 3.0 7.0))
  (bind _returnvalue (AI|SpawnAIFromClass "/Game/TrackDecay/Blueprints/BP_WanderingWoundedMHOptimimized.BP_WanderingWoundedMHOptimimized_C" 0 (+ (Transformation|GetActorLocation) (Math|Vector|MakeVector (Utilities|GetRandomFloatfromBoxExtent (.x _boxextent)) (Utilities|GetRandomFloatfromBoxExtent (.y _boxextent)) 1e+03)) "0, 0, 0" false 0))
  (bind _asbp_wounded (Utilities|Casting|CastToBP_Wounded _returnvalue))
  (Variables|/Game/TrackDecay/Blueprints/BP_Wounded.BP_Wounded_C|SetBoundary _asbp_wounded (Variables|Default|GetBox))
  (Variables|/Game/TrackDecay/Blueprints/BP_Wounded.BP_Wounded_C|SetPlayerColor _asbp_wounded PlayerColor))

(event EventBeginPlay)

(event Collision|EventActorBeginOverlap
  (params (OtherActor :type Actor%20Object%20Reference)))

(event EventTick
  (params (DeltaSeconds :type Float%20%28single-precision%29)))

(fn ConstructionScript)