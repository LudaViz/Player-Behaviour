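; BP_HumanSpawner is a spawner actor that creates BP_Human actors around its location.
; Its SpawnHuman event offsets the actor location per axis by passing the Box extent through GetRandomFloatFromBoxExtent, then always spawns with a random rotation without roll.
; The helper's only node, a random range of plus or minus half the input, is marked unused.
; Nothing in this file calls SpawnHuman.
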(event Custom|SpawnHuman
  (bind _box (Variables|Default|GetBox))
  (bind _boxextent (Variables|/Script/Engine.BoxComponent|GetBoxExtent _box))
  (Game|SpawnActorfromClass "/Game/TrackDecay/BP_Human.BP_Human_C" (Math|Transform|MakeTransform (+ (Transformation|GetActorLocation) (Math|Vector|MakeVector (Utilities|GetRandomFloatfromBoxExtent (.x _boxextent)) (Utilities|GetRandomFloatfromBoxExtent (.y _boxextent)) (Utilities|GetRandomFloatfromBoxExtent (.z _boxextent)))) (Math|Random|RandomRotator false) "1.000000,1.000000,1.000000") "AlwaysSpawn" "MultiplyWithRoot" 0 0))

(event EventBeginPlay)

(event Collision|EventActorBeginOverlap
  (params (OtherActor :type Actor%20Object%20Reference)))

(event EventTick
  (params (DeltaSeconds :type Float%20%28single-precision%29)))

(fn ConstructionScript)