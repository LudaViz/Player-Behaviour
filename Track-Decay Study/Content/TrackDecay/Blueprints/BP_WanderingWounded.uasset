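; BP_WanderingWounded is a pawn that wanders at random within a Boundary volume and leaves mud footprints.
; After BeginPlay it polls until Boundary is valid, then picks navigable points around its X/Y location, using the box's X extent as radius.
; AI MoveTo loops with random pauses after arrival and retries the same destination on failure.
; FootL and FootR events draw left and right mud step brushes while CanMove is true.
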(event Custom|FootL
  (bind _bp_brush_mudstep_l (Variables|Default|GetBP_Brush_MudStep_L))
  ;[0.15 0.15 0.15 0.5] Footprints
  (if (Variables|Default|GetCanMove)
    (Utilities|IsValid _bp_brush_mudstep_l
      (:Is%20Valid
        (Class|InteractBrush|DrawBrush _bp_brush_mudstep_l)))))

(event Custom|FootR
  (bind _bp_brush_mudstep_r (Variables|Default|GetBP_Brush_MudStep_R))
  ;[0.15 0.15 0.15 0.5] Footprints
  (if (Variables|Default|GetCanMove)
    (Utilities|IsValid _bp_brush_mudstep_r
      (:Is%20Valid
        (Class|InteractBrush|DrawBrush _bp_brush_mudstep_r)))))

(event EventBeginPlay
  (bind _boundary (Variables|Default|GetBoundary))
  (bind _returnvalue (Transformation|GetWorldLocation _boundary))
  (Utilities|FlowControl|Delay 0.2)
  (Utilities|IsValid (Variables|Default|GetBoundary) :!label _label
    (:Is%20Valid
      (bind _randomlocation (Class|NavigationSystemV1|GetRandomLocationinNavigableRadius (Math|Vector|MakeVector (.x _returnvalue) (.y _returnvalue) 0.0) (.x (Variables|/Script/Engine.BoxComponent|GetBoxExtent _boundary)) 0 0 :!label _label_2))
      (Variables|Default|SetRandom%20Location _randomlocation)
      (AI|AIMoveTo self (Variables|Default|GetRandom%20Location) 0 5e+01 false :!label _label_3
        (:OnSuccess
          (Utilities|FlowControl|RetriggerableDelay (Math|Random|RandomFloatinRange 1.0 5.0))
          (goto _label_2))
        (:OnFail
          (Utilities|FlowControl|RetriggerableDelay 0.2)
          (goto _label_3))))
    (:Is%20Not%20Valid
      (Utilities|FlowControl|Delay 0.2)
      (goto _label))))

(fn ConstructionScript)