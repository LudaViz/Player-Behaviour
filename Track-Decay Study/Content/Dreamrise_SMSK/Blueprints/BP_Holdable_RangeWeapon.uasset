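; Networked full-auto ranged weapon holdable that fires hitscan shots, reloads from inventory ammo and feeds hand IK to the wielder.
; A looping timer fires locally to hide lag, then the server multicasts effects to other clients.
; Line traces run on each machine, with damage applied only on authority.
; The server saves ammo to the inventory item, while clients update UI, crosshair, hit markers and camera shake.
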(event Custom|Start%20Shooting
  (bind _fire_rate (Variables|Configuration|GetFire%20Rate))
  ;[1 0.4979 0.4979] Local Start Full Auto Shooting, if not reloading continue for Shoot - from Client and To Server to prevent lag
  (bind _returnvalue (Utilities|Time|SetTimerbyEvent (delegate Custom|Shoot) _fire_rate true false (* _fire_rate -1.0)))
  (Variables|Default|SetShooting%20Timer%20Handle _returnvalue))

(event Custom|Stop%20Shooting
  ;[1 0.4833 0.3122] Stop Shooting clear fullauto timer
  (Utilities|Time|ClearandInvalidateTimerbyHandle (Variables|Default|GetShooting%20Timer%20Handle)))

(event Custom|MULTICAST%20Shoot
  (params (Shoot%20Location :type Vector) (Shoot%20Rotation :type Rotator))
  ;[1 0.8733 0.1888] Networked Shooting
  (if (not (CallFunction|IsLocal))
    (CallFunction|LocalShoot Shoot%20Location Shoot%20Rotation)))

(event Custom|CLIENT%20Update%20Ammo
  (params (Current%20Ammo :type Integer))
  (bind _returnvalue (Components|GetOwner))
  ;[0.7421 1 0.6658] Client Update ammo, show it inside Widget
  (Variables|Default|SetCurrent%20Ammo Current%20Ammo)
  (bind _inventory_comp_reference (Class|BPISimpleInventorySystem|BPISimpleInventorySystemGetInventoryComponent(Message) _returnvalue))
  (Utilities|IsValid _inventory_comp_reference
    (:Is%20Valid
      (bind _amount (Default|GetItemAmount _inventory_comp_reference "Ammo"))
      (bind _main_ui (Class|BPIPlayerBase|BPIPlayerBaseGetMainUI(Message) _returnvalue))
      (Class|BPIPlayerUserInterface|BPIPlayerUserInterfaceUpdateAmmo(Message) _main_ui (Variables|Default|GetCurrent%20Ammo) _amount))))

(event Custom|Reload
  ;[1 1 1] Reload on Server
  (Utilities|FlowControl|DoOnce false :!label _label
    (:Completed
      (CallFunction|CLIENTReload)
      (Utilities|FlowControl|Delay (Variables|Configuration|GetReload%20Time))
      (Utilities|FlowControl|Sequence
        (:then_0
          (bind _inventory_comp_reference (Class|BPISimpleInventorySystem|BPISimpleInventorySystemGetInventoryComponent(Message) (Components|GetOwner)))
          (Utilities|IsValid _inventory_comp_reference
            (:Is%20Valid
              ;;[1 1 1] Calculate new ammo if we were possible to remove some from inventory
              (bind (_success _removed_amount) (Default|RemoveItem _inventory_comp_reference "Ammo" (- (Variables|Configuration|GetMax%20Ammo) (Variables|Default|GetCurrent%20Ammo))))
              (if _success
                (bind _output_get (Variables|Default|SetCurrent%20Ammo (+ _removed_amount (Variables|Default|GetCurrent%20Ammo))))
                ;;[1 1 1] Update Ammo inside this weapon
                (CallFunction|CLIENTUpdateAmmo _output_get)
                (CallFunction|ServerUpdateAmmo (Variables|Default|GetCurrent%20Ammo))))))
        (:then_1
          (goto _label Reset))))))

(event Custom|Shoot
  (bind _returnvalue (Game|GetPlayerCameraManager 0))
  (bind _returnvalue_2 (Camera|GetCameraLocation _returnvalue))
  (bind _returnvalue_3 (Camera|GetCameraRotation _returnvalue))
  ;[1 0.4979 0.4979] Local Start Full Auto Shooting, if not reloading continue for Shoot - from Client and To Server to prevent lag
  (if (not (Variables|Default|GetbReloading))
    (CallFunction|LocalShoot _returnvalue_2 _returnvalue_3)
    (CallFunction|SERVERShoot _returnvalue_2 _returnvalue_3)))

(event Custom|CLIENT%20Reload
  ;[1 1 1] Client Reloading
  (Variables|Default|SetbReloading true)
  (Utilities|FlowControl|Sequence
    (:then_0
      ;;[1 1 1] If valid remove prev. widget
      (bind _reloading_widget (Variables|Default|GetReloading%20Widget)
        (:then
          (Widget|RemovefromParent _reloading_widget))
        (:else
          _))
      ;;[1 1 1] Create new action reloading widget
      (bind _returnvalue (UserInterface|CreateWidget "/Game/Dreamrise_SMSK/Blueprints/Widgets/W_Loading.W_Loading_C" 0 (Variables|Configuration|GetReload%20Time)))
      (bind _output_get (Variables|Default|SetReloading%20Widget _returnvalue))
      (UserInterface|Viewport|AddtoViewport _output_get -1))
    (:then_1
      ;;[1 1 1] Expire reloading
      (Utilities|FlowControl|Delay (Variables|Configuration|GetReload%20Time))
      (Variables|Default|SetbReloading false))))

(event Custom|Local%20Shoot
  (params (Shoot%20Location :type Vector) (Shoot%20Rotation :type Rotator))
  (bind _returnvalue (Game|GetPlayerController 0))
  (bind _staticmesh (Variables|Default|GetStaticMesh))
  (bind _staticmesh_2 (Variables|Default|GetStaticMesh))
  (bind _returnvalue_2 (Transformation|GetSocketLocation _staticmesh "BarrelSocket"))
  ;[0.1751 0.8519 1] Local On Shoot, Play some effects, apply damage
  (if (> (Variables|Default|GetCurrent%20Ammo) 0)
    (Utilities|FlowControl|Sequence
      (:then_0
        (Effects|SpawnEmitterAttached "/Game/Dreamrise_SMSK/Assets/FX/P_Gunshot.P_Gunshot" _staticmesh_2 "None" _returnvalue_2 "0, 0, 0" "1.000000,1.000000,1.000000" "KeepWorldPosition" true "AutoRelease")
        (Audio|SpawnSoundAttached (Variables|Configuration|GetGunshot%20Sound) _staticmesh_2 "None" _returnvalue_2 "0, 0, 0" "KeepWorldPosition" false 1.0 1.0 0.0 "/Game/Dreamrise_SMSK/Audio/Attenuation/SAT_Gunshot.SAT_Gunshot" "/Game/Dreamrise_SMSK/Audio/Concurency/SC_Gunshot.SC_Gunshot")
        (Math|Integer|DecrementInt (Variables|Default|GetCurrent%20Ammo)
          (:%20%20
            (bind (_outhit _returnvalue_3) (Collision|LineTraceForObjects Shoot%20Location (+ Shoot%20Location (* (Math|Vector|GetForwardVector Shoot%20Rotation) (Math|Float|MakeLiteralFloat 1e+04))) (Utilities|Array|MakeArray "ObjectTypeQuery1" "ObjectTypeQuery3" "ObjectTypeQuery4") false (Utilities|Array|MakeArray (Game|GetInstigator)) "None"))
            (if _returnvalue_3
              (Effects|SpawnEmitteratLocation "/Game/Dreamrise_SMSK/Assets/FX/P_ImpactStuff.P_ImpactStuff" (.ImpactPoint (Collision|BreakHitResult _outhit)) "0, 0, 0" "1.000000,1.000000,1.000000" true "AutoRelease")
              (Utilities|FlowControl|Sequence
                (:then_0
                  (Networking|SwitchHasAuthority
                    (:Authority
                      (Game|Damage|ApplyDamage (.HitActor (Collision|BreakHitResult _outhit)) (Variables|Configuration|GetDamage) (Game|GetInstigatorController) self)
                      ;;[1 1 1] Server Failsafe set ammo
                      (CallFunction|CLIENTUpdateAmmo (Variables|Default|GetCurrent%20Ammo) :!label _label)
                      (CallFunction|ServerUpdateAmmo (Variables|Default|GetCurrent%20Ammo)))))
                (:then_1
                  (if (CallFunction|IsLocal)
                    (Utilities|IsValid (.HitActor (Collision|BreakHitResult _outhit))
                      (:Is%20Valid
                        (if (Variables|/Script/Engine.Actor|GetbCanBeDamaged (.HitActor (Collision|BreakHitResult _outhit)))
                          (bind _main_ui (Class|BPIPlayerBase|BPIPlayerBaseGetMainUI(Message) (Components|GetOwner)))
                          (Class|BPIHoldable|BPIHoldableonHit(Message) _main_ui)))))))
              (else
                (goto _label))))))
      (:then_1
        ;;[1 1 1] Play Anim Blueprint Animation
        (bind _ascharacter (Utilities|Casting|CastToCharacter (Game|GetInstigator)))
        (bind _asabp_manny (Utilities|Casting|CastToABP_Manny (Components|SkeletalMesh|GetAnimInstance (Variables|/Script/Engine.Character|GetMesh _ascharacter))))
        (Default|Shoot _asabp_manny (Variables|Configuration|GetShoot%20Intensity)))
      (:then_2
        ;;[1 1 1] Play Camera Shake on Local Client
        (if (CallFunction|IsLocal)
          (Game|Feedback|ClientStartCameraShake _returnvalue "/Game/Dreamrise_SMSK/Other/Camera/CMS_Shoot.CMS_Shoot_C" (Math|Float|MapRangeClamped (Variables|Configuration|GetShoot%20Intensity) 1e+01 5e+01 1.0 2.5) "CameraLocal" "0, 0, 0")
          (bind _main_ui_2 (Class|BPIPlayerBase|BPIPlayerBaseGetMainUI(Message) _returnvalue))
          (Class|BPIHoldable|BPIHoldableonShoot(Message) _main_ui_2 (Utilities|Struct|BreakS_Holdable_Crosshair (Variables|Configuration|GetCrosshair)))
          (Class|PlayerController|AddPitchInput _returnvalue -0.3))))))

(event Custom|SERVER%20Shoot
  (params (Shoot%20Location :type Vector) (Shoot%20Rotation :type Rotator))
  ;[1 0.8733 0.1888] Networked Shooting
  (if (> (Variables|Default|GetCurrent%20Ammo) 0)
    (CallFunction|MULTICASTShoot Shoot%20Location Shoot%20Rotation)))

(event EventDestroyed
  ;[1 1 1] On Destroyed
  (|CallParentFunction)
  (|CGraph_Destroyed))

(event EventTick
  (params (DeltaSeconds :type Float%20%28single-precision%29))
  ;[1 1 1] Tick, update Hand IK
  (|CallParentFunction DeltaSeconds)
  (|CGraph_Tick))

(event EventBeginPlay
  ;[1 1 1] On Begin Play
  (|CallParentFunction)
  (|CGraph_BeginPlay))

(fn ConstructionScript
  (|CallParentFunction))

(fn BPIHoldableCallHoldableAction
  (params (Action :type Name :default "None"))
  (switch name Action
    (:Default
      (return false))
    (:StartPrimary
      (CallFunction|StartShooting))
    (:StopPrimary
      (CallFunction|StopShooting))
    (:Reload
      (CallFunction|Reload)))
  (return true))

(fn BPIHoldableGetCrosshairData
  (return (Variables|Configuration|GetCrosshair)))

(fn ServerUpdateAmmo
  (params (Current%20Ammo :type Integer))
  (Networking|SwitchHasAuthority
    (:Authority
      (Variables|Default|SetCurrent%20Ammo Current%20Ammo)
      (bind _inventory_comp_reference (Class|BPISimpleInventorySystem|BPISimpleInventorySystemGetInventoryComponent(Message) (Components|GetOwner)))
      (Utilities|IsValid _inventory_comp_reference
        (:Is%20Valid
          (Default|ModifyItemAmmo _inventory_comp_reference (Variables|Default|GetItem%20ID) (Variables|Default|GetCurrent%20Ammo) false)
          (return))))))

(fn BPIHoldableGetAmmoData
  (return true 0))

(event Custom|On%20Inventory%20Item%20Updated
  ;[1 0.5271 0.886] Update Ammo when Inventory gets updated (for example player obtains more ammo)
  (CallFunction|CLIENTUpdateAmmo (Variables|Default|GetCurrent%20Ammo)))