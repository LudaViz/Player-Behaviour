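; Holdable build hammer that lets the local player preview and place a building of a set class.
; On BeginPlay it spawns a local ghost and recipe requirement widget, both removed on destroy.
; Each tick a camera line trace against WorldStatic positions the ghost and sets whether building is allowed.
; Holdable interface scroll actions rotate it, and primary sends class, transform and recipe to the player controller's server build request.
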(event Custom|Try%20to%20Build
  ;[1 1 1] Try to Build
  (if (Variables|Default|GetbCanBuild)
    (bind _asbp_track_decay_player_controller (Utilities|Casting|CastToBP_TDS_PlayerController (Game|GetPlayerController 0)))
    (bind _result (Utilities|Set|ToArray (Variables|Configuration|GetRecipe)))
    (Default|SEVRERRequestBuild _asbp_track_decay_player_controller (Variables|Configuration|GetBuilding%20Class) (Transformation|GetActorTransform (Variables|Default|GetLocally%20Spawned%20Build)) _result)))

(event EventBeginPlay
  ;[1 1 1] Spawn Building Ghost on Local for Building
  (|CallParentFunction)
  (if (CallFunction|IsLocal)
    (bind _returnvalue (Game|SpawnActorfromClass (Variables|Configuration|GetBuilding%20Class) (Math|Transform|MakeTransform "0, 0, 0" "0, 0, 0" "1.000000,1.000000,1.000000") "AlwaysSpawn" "MultiplyWithRoot" 0 true 5e+02 0))
    (Variables|Default|SetLocally%20Spawned%20Build _returnvalue)
    ;[1 1 1] Create recipe widget
    (bind _result (Utilities|Set|ToArray (Variables|Configuration|GetRecipe)))
    (bind _returnvalue_2 (UserInterface|CreateWidget "/Game/Dreamrise_SMSK/Blueprints/Widgets/W_BuildingRequirement.W_BuildingRequirement_C" 0 _result))
    (bind _output_get (Variables|Default|SetRequirement%20Widget _returnvalue_2))
    (UserInterface|Viewport|AddtoViewport _output_get -1)))

(event EventTick
  (params (DeltaSeconds :type Float%20%28single-precision%29))
  (bind _returnvalue (Game|GetPlayerCameraManager 0))
  (bind _locally_spawned_build (Variables|Default|GetLocally%20Spawned%20Build))
  (bind _returnvalue_2 (Camera|GetCameraLocation _returnvalue))
  ;[1 1 1] Adjust local building actor transform
  (|CallParentFunction DeltaSeconds)
  (if (CallFunction|IsLocal)
    (bind (_outhit _returnvalue_3) (Collision|LineTraceForObjects _returnvalue_2 (+ (* (Math|Vector|GetForwardVector (Camera|GetCameraRotation _returnvalue)) (Math|Float|MakeLiteralFloat 1.5e+03)) _returnvalue_2) (Utilities|Array|MakeArray "ObjectTypeQuery1") false 0 "None"))
    (Variables|Default|SetbCanBuild _returnvalue_3)
    (Transformation|SetActorLocation _locally_spawned_build (select _returnvalue_3 (.ImpactPoint (Collision|BreakHitResult _outhit)) (.TraceEnd (Collision|BreakHitResult _outhit))) false false)
    (Transformation|SetActorRotation _locally_spawned_build (Math|Rotator|MakeRotator 0.0 0.0 (Variables|Default|GetBuild%20Rotation%20Z)))))

(event EventDestroyed
  ;[1 1 1] Destroy Building Ghost
  (|CallParentFunction)
  (Utilities|FlowControl|Sequence
    (:then_0
      (bind _locally_spawned_build (Variables|Default|GetLocally%20Spawned%20Build)
        (:then
          (Actor|DestroyActor _locally_spawned_build))
        (:else)))
    (:then_1
      (bind _requirement_widget (Variables|Default|GetRequirement%20Widget)
        (:then
          (Widget|RemovefromParent _requirement_widget))
        (:else)))))

(fn ConstructionScript
  (|CallParentFunction))

(fn BPIHoldableCallHoldableAction
  (params (Action :type Name :default "None"))
  (switch name Action
    (:Default
      (return false))
    (:ScrollUp
      (Variables|Default|SetBuild%20Rotation%20Z (+ (Variables|Default|GetBuild%20Rotation%20Z) 5.0)))
    (:ScrollDown
      (Variables|Default|SetBuild%20Rotation%20Z (+ (Variables|Default|GetBuild%20Rotation%20Z) -5.0)))
    (:StartPrimary
      (CallFunction|TrytoBuild)))
  (return true))